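; BP_Nest is a spawner actor that produces a turtle AI pawn when its Spawn event is called.
; Spawn plays a sound and adds a particle effect, then spawns the configured pawn class at the nest's root, ignoring collision.
; It casts the pawn's controller to BP_AIController_Turtle and calls Move, handing over the nest's editable start and end targets plus run, idle and run-back times.
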(event `Spawn`
  (bind _returnvalue (`SceneComponent.K2_GetComponentLocation` (`self.DefaultSceneRoot`)))
  ; Sound and visual effects
  (`GameplayStatics.PlaySoundAtLocation` "/Game/Project/Sounds/SpawnGnomeWoo.SpawnGnomeWoo" _returnvalue (struct) 1.0 1.0 0.0 null null null null)
  (`AddComponent|NODE_AddParticleSystemComponent-0`)
  ; Spawn Turtle
  (bind _returnvalue_2 (`AIBlueprintHelperLibrary.SpawnAIFromClass` (`self.AI Pawn Class`) null _returnvalue (struct) true null))
  (bind _asbp_aicontroller_turtle (cast `/Game/Project/Blueprints/BP_AIController_Turtle` (`AIBlueprintHelperLibrary.GetAIController` _returnvalue_2)))
  (`/Game/Project/Blueprints/BP_AIController_Turtle.Move` _asbp_aicontroller_turtle _returnvalue_2 (`self.Target End`) (`self.Run Time`) (`self.Idle Time`) (`self.Target Start`) (`self.Run Back Time`)))

(fn `UserConstructionScript`)